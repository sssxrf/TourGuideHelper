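; BP_PathFinal is a spline-based path actor that draws a thin mesh strip along its spline, hidden by default.
; Its construction script adds a scaled-down spline mesh for each segment between neighboring points, fitted to their local locations and tangents, and stores them in SplineMeshes.
; Events loop over that array to show or hide the path, or to switch every segment to the Mat_PathFinal material when a path change is confirmed.
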(event `ConfirmChangePathMat`
  (for _array_element (`self.SplineMeshes`)
    (`PrimitiveComponent.SetMaterial` _array_element 0 "/Game/TGH/Path/Mat_PathFinal.Mat_PathFinal")))

(event `ShowSplineMesh`
  (for _array_element (`self.SplineMeshes`)
    (`SceneComponent.SetVisibility` _array_element true false)))

(event `HideSplineMesh`
  (for _array_element (`self.SplineMeshes`)
    (`SceneComponent.SetVisibility` _array_element false false)))

(fn `UserConstructionScript`
  (bind _spline (`self.Spline`))
  (for _index (range (+ (- (`SplineComponent.GetNumberOfSplinePoints` (`self.Spline`)) 2) 1))
    (bind _returnvalue (`AddComponent|NODE_AddSplineMeshComponent-0`))
    (`KismetArrayLibrary.Array_Add` (`self.SplineMeshes`) _returnvalue)
    (`SceneComponent.K2_AttachToComponent` _returnvalue (`self.DefaultSceneRoot`) "None" "KeepRelative" "KeepRelative" "KeepRelative" true)
    (bind (_location _tangent) (`SplineComponent.GetLocationAndTangentAtSplinePoint` _spline _index "Local"))
    (bind (_location_2 _tangent_2) (`SplineComponent.GetLocationAndTangentAtSplinePoint` _spline (+ _index 1) "Local"))
    (`SplineMeshComponent.SetStartAndEnd` _returnvalue _location _tangent _location_2 _tangent_2 true)
    (`SplineMeshComponent.SetStartScale` _returnvalue (0.1 0.1) true)
    (`SplineMeshComponent.SetEndScale` _returnvalue (0.1 0.1) true)
    (`SceneComponent.SetVisibility` _returnvalue false false)))