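; BP_DayPlanShop is the shop entry of a day plan, a cube with a GrabComponent that snaps into the cafe entry's stored position when dropped.
; On BeginPlay it saves the cube's world transform as CurrentTransformShop and caches the BP_DayPlanCafe actor found in the level.
; On drop it reads CurrentTransformCafe from that actor and moves the cube there without sweep, with no proximity check.
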(event `self.ReceiveBeginPlay`
  (set `self.CurrentTransformShop` (`SceneComponent.K2_GetComponentToWorld` (`self.Cube`)))
  (bind _returnvalue (`GameplayStatics.GetActorOfClass` "/Game/TGH/BP/BP_DayPlanCafe.BP_DayPlanCafe_C"))
  (set `self.Cafe` _returnvalue))

(event `self.GrabComponent.OnDropped`
  (set `self.TargetTransformShop` (`/Game/TGH/BP/BP_DayPlanCafe.CurrentTransformCafe` (`self.Cafe`)))
  (`SceneComponent.K2_SetWorldTransform` (`self.Cube`) (`self.TargetTransformShop`) false false))

(fn `UserConstructionScript`)