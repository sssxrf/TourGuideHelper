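; BP_Car is a car Blueprint that travels along the spline of a BP_PathFinal actor.
; On BeginPlay it finds and stores that path actor.
; The MoveCar event plays a timeline at a rate of 1/TimeToComplete, mapping its track to spline distance to set the Car's world location and rotation.
; Nothing in this graph triggers MoveCar, as its only call here is disconnected.
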(event `self.ReceiveBeginPlay`
  (bind _returnvalue (`GameplayStatics.GetActorOfClass` "/Game/TGH/Path/BP_PathFinal.BP_PathFinal_C"))
  (set `self.PathFinal` _returnvalue))

(event `MoveCar`
  (bind _spline (`/Game/TGH/Path/BP_PathFinal.Spline` (`self.PathFinal`)))
  (`TimelineComponent.SetPlayRate` (`self.CarMoveTimeline`) (/ 1.0 (`self.TimeToComplete`)))
  (bind (_direction _movetrack) (`Timeline|CarMoveTimeline`)
    (:`Update`
      (bind _returnvalue (`KismetMathLibrary.Lerp` 0.0 (`SplineComponent.GetSplineLength` (`/Game/TGH/Path/BP_PathFinal.Spline` (`self.PathFinal`))) _movetrack))
      (`SceneComponent.K2_SetWorldLocationAndRotation` (`self.Car`) (`SplineComponent.GetLocationAtDistanceAlongSpline` _spline _returnvalue "World") (`SplineComponent.GetRotationAtDistanceAlongSpline` _spline _returnvalue "World") false false))))

(fn `UserConstructionScript`)