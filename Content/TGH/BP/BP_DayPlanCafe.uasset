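; BP_DayPlanCafe is an actor, apparently the cafe piece of a day-plan arrangement, that snaps its cube to the shop piece's position.
; On BeginPlay it stores its cube's world transform in CurrentTransformCafe and finds the BP_DayPlanShop instance.
; When its Box overlaps an actor tagged "Shop", the cube takes that cached instance's CurrentTransformShop.
; The stored cafe transform is never updated after the move.
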(event `self.ReceiveBeginPlay`
  (set `self.CurrentTransformCafe` (`SceneComponent.K2_GetComponentToWorld` (`self.Cube`)))
  (bind _returnvalue (`GameplayStatics.GetActorOfClass` "/Game/TGH/BP/BP_DayPlanShop.BP_DayPlanShop_C"))
  (set `self.Shop` _returnvalue))

(event `self.Box.OnComponentBeginOverlap`
  (params (OverlappedComponent :type "PrimitiveComponent Object Reference") (OtherActor :type "Actor Object Reference") (OtherComp :type "PrimitiveComponent Object Reference") (OtherBodyIndex :type Integer) (bFromSweep :type Boolean) (SweepResult :type "HitResult Structure (by ref)"))
  (if (`self.ActorHasTag` OtherActor "Shop")
    (set `self.TargetTransform` (`/Game/TGH/BP/BP_DayPlanShop.CurrentTransformShop` (`self.Shop`)))
    (`SceneComponent.K2_SetWorldTransform` (`self.Cube`) (`self.TargetTransform`) false false)))

(fn `UserConstructionScript`)